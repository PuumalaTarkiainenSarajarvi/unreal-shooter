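; BP_BazookaWeapon is a bazooka weapon that fires missile projectiles.
; On PullTrigger it calls DecrementAmmo and, if that succeeds, spawns a BP_MissileProjectile at the ProjectileSpawnPoint transform.
; It then plays the Laser_hit sound at the weapon's location, except when the game mode is BP_MainMenuGamemode, where firing stays silent.
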(event `self.PullTrigger`
  (params (Instigator :type "Controller Object Reference"))
  (bind _returnvalue_location (`KismetMathLibrary.BreakTransform` (`self.GetTransform`)))
  ;[1 1 1] Firing logic
  (bind _return_value (`self.DecrementAmmo`))
  (if _return_value
    (`|SpawnActorFromClass` "/Game/Blueprints/BP_MissileProjectile.BP_MissileProjectile_C" (`SceneComponent.K2_GetComponentToWorld` (`self.ProjectileSpawnPoint`)) "Undefined" "OverrideRootScale" null null)
    (cast `/Game/Blueprints/BP_MainMenuGamemode` (`GameplayStatics.GetGameMode`)
      (:`CastFailed`
        (`GameplayStatics.PlaySoundAtLocation` "/Game/Sounds/laser_hit.laser_hit" _returnvalue_location (struct) 1.0 1.0 0.0 null null null)))))

(fn `UserConstructionScript`
  (`parent.UserConstructionScript`))