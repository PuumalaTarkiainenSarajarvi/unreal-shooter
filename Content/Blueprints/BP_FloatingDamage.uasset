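; Floating damage number actor that shows a damage value as dark red rising text, then destroys itself after AliveTime.
; ServerSetDamageText forwards the value to MultiSetDamageText, a server-to-multicast style relay that sets the TextRender to the rounded number.
; Tick calls MoveComponentTo every frame to lift and rotate the text toward a fixed relative offset, while a timer started on BeginPlay handles destruction.
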(event `self.ReceiveBeginPlay`
  ;[1 1 1] Should be destroyed after some time
  (`/Engine/EditorBlueprintResources/StandardMacros.DoOnce` false :!label _label
    (:`Completed`
      (`KismetSystemLibrary.K2_SetTimer` null "DestroySelf" (`self.AliveTime`)))))

(event `DestroySelf`
  ;[1 1 1] Should be destroyed after some time
  (`self.K2_DestroyActor`)
  (goto _label :!via `Reset`))

(event `ServerSetDamageText`
  (params (Damage :type "Float (double-precision)"))
  ;[1 1 1] Set Damage text
  (`self.MultiSetDamageText` Damage))

(event `MultiSetDamageText`
  (params (Damage :type "Float (double-precision)"))
  ;[1 1 1] Set Damage text
  (`TextRenderComponent.K2_SetText` (`self.TextRender`) (`KismetTextLibrary.Conv_Int64ToText` (`KismetMathLibrary.Round64` Damage))))

(event `self.ReceiveTick`
  (params (DeltaSeconds :type "Float (single-precision)"))
  (`KismetSystemLibrary.MoveComponentTo` (`self.TextRender`) (0.0 0.0 100.0) (struct :`Roll` 90.0) false false 1.0))

(event `self.TextRender.OnComponentWake`
  (params (WakingComponent :type "PrimitiveComponent Object Reference") (BoneName :type Name)))

(fn `UserConstructionScript`
  (`TextRenderComponent.SetTextRenderColor` (`self.TextRender`) (`KismetMathLibrary.Conv_LinearColorToColor` (struct :`R` 0.276042 :`B` 0.001701 :`A` 1.0))))