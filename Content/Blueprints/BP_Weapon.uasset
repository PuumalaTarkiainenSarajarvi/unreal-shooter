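; Weapon actor that fires BP_Projectile automatically while the trigger is held and carries an attached laser sight.
; PullTrigger passes a DoOnce gate to fire immediately and start a looping timer at RoundsPerSecond, while ReleaseTrigger clears the timer and resets the gate.
; BeginPlay switches on authority, calling MultiSpawnLaser directly or through ServerSpawnLaser, to spawn the laser sight and snap it to WeaponMesh.
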(event `MultiSpawnLaser`
  (bind _weaponmesh (`self.WeaponMesh`))
  (bind _output_get (set `self.WeaponWorldTransform` (`SceneComponent.K2_GetComponentToWorld` _weaponmesh)))
  (bind _returnvalue (`|SpawnActorFromClass` "/Game/Blueprints/BP_LaserSight.BP_LaserSight_C" _output_get "Undefined" "OverrideRootScale" null null))
  (`self.K2_AttachToComponent` _returnvalue _weaponmesh "None" "SnapToTarget" "KeepRelative" "SnapToTarget" true)
  (`KismetSystemLibrary.PrintString` "Spawned laser"))

(event `ServerSpawnLaser`
  (`self.MultiSpawnLaser`))

(event `self.ReceiveBeginPlay`
  (`/Engine/EditorBlueprintResources/ActorMacros.Switch Has Authority`
    (:`Authority`
      (`self.MultiSpawnLaser`))
    (:`Remote`
      (`self.ServerSpawnLaser`))))

(event `PullTrigger`
  ;[1 1 1] Trigger pulling & releasing timer logic
  (`/Engine/EditorBlueprintResources/StandardMacros.DoOnce` false :!label _label
    (:`Completed`
      (`self.FireWeapon`)
      (`KismetSystemLibrary.K2_SetTimer` null "FireWeapon" (/ 1.0 (`self.RoundsPerSecond`)) true))))

(event `ReleaseTrigger`
  ;[1 1 1] Trigger pulling & releasing timer logic
  (`KismetSystemLibrary.K2_ClearTimer` null "FireWeapon")
  (goto _label :!via `Reset`))

(event `FireWeapon`
  ;[1 1 1] Weapon firing & spawning projectile
  (`|SpawnActorFromClass` "/Game/Blueprints/BP_Projectile.BP_Projectile_C" (`SceneComponent.K2_GetComponentToWorld` (`self.ProjectileSpawnPoint`)) "Undefined" "OverrideRootScale" null null))

(fn `UserConstructionScript`)