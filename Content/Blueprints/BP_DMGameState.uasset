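; Deathmatch game state that runs the round countdown, tracks connected players and handles map voting and session shutdown.
; When time expires, it ends the game via SideScrollerGameMode, builds score-sorted player stats on authority, then shows game-over scores after a short, unconditional delay.
; RepNotify player and vote data feed change dispatchers, with votes moved between maps on change.
; Server teardown destroys each player's session and opens the main menu.
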(event `TimerCountdown`
  ;[1 1 1] Round timer
  (bind _result (`/Engine/EditorBlueprintResources/StandardMacros.DecrementInt` (`self.RoundTime`))
    (:`  `
      (bind _output_get (set `self.RoundTime` _result))
      (if (<= _output_get 0)
        (`self.SetGameEnded`)
        (`self.GetConnectedPlayerData`)
        (`KismetSystemLibrary.K2_ClearTimer` null "TimerCountdown")
        (goto _label :!via `Reset`)))))

(event `self.ReceiveBeginPlay`
  ;[1 1 1] Round timer
  (`/Engine/EditorBlueprintResources/StandardMacros.DoOnce` false :!label _label
    (:`Completed`
      (`KismetSystemLibrary.K2_SetTimer` null "TimerCountdown" 1.0 true))))

(event `ShowEndScores`
  (bind _asside_scroller_game_mode (cast `/Game/SideScrollerBP/Blueprints/SideScrollerGameMode` (`GameplayStatics.GetGameMode`)))
  (`/Game/SideScrollerBP/Blueprints/SideScrollerGameMode.ShowGameOverScreen` _asside_scroller_game_mode))

(event `SetGameEnded`
  (bind _asside_scroller_game_mode (cast `/Game/SideScrollerBP/Blueprints/SideScrollerGameMode` (`GameplayStatics.GetGameMode`)))
  (`/Game/SideScrollerBP/Blueprints/SideScrollerGameMode.SetGameEnded` _asside_scroller_game_mode))

(event `GetConnectedPlayerData`
  (`/Engine/EditorBlueprintResources/ActorMacros.Switch Has Authority`
    (:`Authority`
      (`self.GetPlayerInfoForStatistics`)
      (`KismetSystemLibrary.Delay` 0.1)
      (`self.IsEndGameInfoReady`))))

(event `MapVoted`
  (`self.MapVotesUpdated` (`self.MapVotes`)))

(event `DisconnectPlayer`
  (params (LeavingPlayer :type "PlayerController Object Reference"))
  (`DestroySessionCallbackProxy.DestroySession` LeavingPlayer
    (:`OnSuccess`
      _)
    (:`OnFailure`
      _))
  (`GameplayStatics.OpenLevel` "_MainMenu"))

(event `DestroyServer`
  (`self.DisconnectAllPlayers` (`self.ConnectedPlayers`)))

(event `ServerRunVote`
  (params (LastVotedMap :type Name) (NewVotedMap :type Name))
  (`self.UpdateMapVotes` LastVotedMap NewVotedMap))

(fn `DisconnectAllPlayers`
  (params (ConnectedPlayers :type "Array of /Game/Blueprints/ConnectedPlayerInfoStructure Structure"))
  (locals (PlayersToDisconnect :type "Array of /Game/Blueprints/ConnectedPlayerInfoStructure Structure"))
  (bind _output_get (set `local.PlayersToDisconnect` ConnectedPlayers))
  (for _array_element _output_get
    (`self.DisconnectPlayer` (break `/Game/Blueprints/ConnectedPlayerInfoStructure` _array_element))))

(fn `GetPlayerInfoForStatistics`
  (for _array_element (`self.ConnectedPlayers`)
    (bind _asbp_player_state (cast `/Game/Blueprints/BP_PlayerState` (`Controller.PlayerState` (break `/Game/Blueprints/ConnectedPlayerInfoStructure` _array_element))))
    (`KismetArrayLibrary.Array_Add` (`self.GameEndPlayerInfo`) (make `PlayerData` (`.PlayerName_5_E918BB484E6660929CACC7A75CDA77FB` (break `/Game/Blueprints/ConnectedPlayerInfoStructure` _array_element)) (`/Game/Blueprints/BP_PlayerState.PlayerScore` _asbp_player_state))))
  (bind _sorted_array (`ArraySort.PlayerData_Sort` (`self.GameEndPlayerInfo`) true))
  (set `self.GameEndPlayerInfo` _sorted_array))

(fn `IsEndGameInfoReady`
  (if true
    (`KismetSystemLibrary.K2_ClearTimer` null "IsEndGameInfoReady")
    (`self.ShowEndScores`)))

(fn `OnRep_ConnectedPlayers`
  (`self.ConnectedPlayersChanged` (`self.ConnectedPlayers`)))

(fn `OnRep_MapVotes`
  (`self.MapVotesUpdated` (`self.MapVotes`)))

(fn `PlayerJoin`
  (params (JoinedPlayer :type "PlayerController Object Reference"))
  (bind _asbp_player_state (cast `/Game/Blueprints/BP_PlayerState` (`Controller.PlayerState` JoinedPlayer)))
  (`KismetArrayLibrary.Array_Add` (`self.ConnectedPlayers`) (make `/Game/Blueprints/ConnectedPlayerInfoStructure` JoinedPlayer (`/Game/Blueprints/BP_PlayerState.OnlinePlayerName` _asbp_player_state)))
  (set `self.ConnectedPlayers` (`self.ConnectedPlayers`)))

(fn `PlayerLeave`
  (params (LeavingPlayer :type "PlayerController Object Reference"))
  (`KismetArrayLibrary.Array_RemoveItem` (`self.ConnectedPlayers`) (make `/Game/Blueprints/ConnectedPlayerInfoStructure` LeavingPlayer (`/Game/Blueprints/BP_PlayerState.OnlinePlayerName` (cast `/Game/Blueprints/BP_PlayerState` (`Controller.PlayerState` LeavingPlayer) :!pure true))))
  (set `self.ConnectedPlayers` (`self.ConnectedPlayers`)))

(fn `UpdateMapVotes`
  (params (LastVotedMap :type Name :default "null") (NewVotedMap :type Name))
  (locals (NewMapIndex :type Integer) (MapsArray :type "Array of Name") (VotesArray :type "Array of Integer") (LastMapIndex :type Integer))
  (bind (_maps _votes) (break `/Game/Blueprints/MapVotesStructure` (`self.MapVotes`)))
  (bind _returnvalue (- (`|GetArrayItem` (`local.VotesArray`) (`local.LastMapIndex`)) 1))
  (`KismetSystemLibrary.PrintString` (`KismetStringLibrary.Concat_StrStr` (`KismetStringLibrary.Conv_NameToString` LastVotedMap) (`KismetStringLibrary.Conv_NameToString` NewVotedMap) " was voted") true true (struct :`R` 1.0 :`G` 0.09129 :`A` 1.0))
  (set `local.MapsArray` _maps)
  (set `local.VotesArray` _votes)
  (set `local.NewMapIndex` (`KismetArrayLibrary.Array_Find` (`local.MapsArray`) (`local.NewVotedMap`)))
  (set `local.LastMapIndex` (`KismetArrayLibrary.Array_Find` (`local.MapsArray`) (`local.LastVotedMap`)))
  (if (== (`local.LastVotedMap`) "null")
    (`KismetArrayLibrary.Array_Set` (`local.VotesArray`) (`local.NewMapIndex`) (+ (`|GetArrayItem` (`local.VotesArray`) (`local.NewMapIndex`)) 1))
    (else
      (if (< _returnvalue 0)
        (`KismetArrayLibrary.Array_Set` (`local.VotesArray`) (`local.LastMapIndex`))
        (else
          (`KismetArrayLibrary.Array_Set` (`local.VotesArray`) (`local.LastMapIndex`) _returnvalue)))
      (`KismetArrayLibrary.Array_Set` (`local.VotesArray`) (`local.NewMapIndex`) (+ (`|GetArrayItem` (`local.VotesArray`) (`local.NewMapIndex`)) 1))))
  (set `self.MapVotes` (make `/Game/Blueprints/MapVotesStructure` (`local.MapsArray`) (`local.VotesArray`))))

(fn `UserConstructionScript`)