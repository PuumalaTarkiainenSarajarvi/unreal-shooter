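; BP_BaseLinetraceWeapon is a base hitscan weapon that deals damage to whatever its line trace hits.
; PullTrigger traces from the FireDirection component against pawns and world objects, ending a fixed distance along that component's forward vector, measured from the root's location.
; It applies BaseDamage to the hit actor with itself as the damage causer, without checking the hit result.
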(event `self.PullTrigger`
  (bind _firedirection (`self.FireDirection`))
  (bind _outhit (`KismetSystemLibrary.LineTraceSingleForObjects` (`SceneComponent.K2_GetComponentLocation` _firedirection) (+ (`SceneComponent.K2_GetComponentLocation` (`self.DefaultSceneRoot`)) (* (`SceneComponent.GetForwardVector` _firedirection) 2000.0)) (`|MakeArray` "ObjectTypeQuery3" "ObjectTypeQuery2" "ObjectTypeQuery1" :!type "EObjectTypeQuery Enum")))
  (`GameplayStatics.ApplyDamage` (`.HitActor` (`GameplayStatics.BreakHitResult` _outhit)) (`self.BaseDamage`) null self))

(fn `UserConstructionScript`
  (`parent.UserConstructionScript`))