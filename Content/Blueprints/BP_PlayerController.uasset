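; Player controller Blueprint that drives the end-of-match screens and relays map votes for a deathmatch game.
; It shows a statistics widget, then after a delay swaps to a host or client lobby widget based on authority.
; Vote requests go directly or through RequestVoteFromServer to update BP_DMGameState.
; Update requests refresh voted maps only when the current widget is the host lobby.
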(event `ShowEndGameScreen`
  (bind _returnvalue (`|CreateWidget` "/Game/Widgets/BP_EndGameStatistics.BP_EndGameStatistics_C"))
  (set `self.EndGameWidget` _returnvalue)
  (`WidgetLayoutLibrary.RemoveAllWidgets`)
  (`UserWidget.AddToViewport` _returnvalue 0)
  (`KismetSystemLibrary.Delay` (`self.TimeToShowEndGameStatistics`))
  (`/Engine/EditorBlueprintResources/ActorMacros.Switch Has Authority`
    (:`Authority`
      (bind _returnvalue_2 (`|CreateWidget` "/Game/Widgets/BP_EndGameLobby_Host.BP_EndGameLobby_Host_C"))
      (set `self.EndGameWidget` _returnvalue_2)
      (`WidgetLayoutLibrary.RemoveAllWidgets`)
      (`UserWidget.AddToViewport` _returnvalue_2 0))
    (:`Remote`
      (bind _returnvalue_3 (`|CreateWidget` "/Game/Widgets/BP_EndGameLobby_Client.BP_EndGameLobby_Client_C"))
      (set `self.EndGameWidget` _returnvalue_3)
      (`WidgetLayoutLibrary.RemoveAllWidgets`)
      (`UserWidget.AddToViewport` _returnvalue_3 0))))

(event `UpdateMapVotes`
  (bind _asbp_end_game_lobby_host (cast `/Game/Widgets/BP_EndGameLobby_Host` (`self.EndGameWidget`)))
  (`/Game/Widgets/BP_EndGameLobby_Host.UpdateVotedMaps` :`self` _asbp_end_game_lobby_host))

(event `RequestMapVoteUpdate`
  (`self.UpdateMapVotes`))

(event `RequestMapVote`
  (params (LastVotedMap :type Name) (NewVotedMap :type Name))
  (`/Engine/EditorBlueprintResources/ActorMacros.Switch Has Authority`
    (:`Authority`
      (`self.ServerRunVote` LastVotedMap NewVotedMap))
    (:`Remote`
      (`self.RequestVoteFromServer` LastVotedMap NewVotedMap))))

(event `RequestVoteFromServer`
  (params (LastVotedMap :type Name) (NewVotedMap :type Name))
  (`self.ServerRunVote` LastVotedMap NewVotedMap))

(event `ServerRunVote`
  (params (LastVotedMap :type Name) (NewVotedMap :type Name))
  (bind _asbp_dmgame_state (cast `/Game/Blueprints/BP_DMGameState` (`GameplayStatics.GetGameState`)))
  (`/Game/Blueprints/BP_DMGameState.UpdateMapVotes` _asbp_dmgame_state LastVotedMap NewVotedMap))

(fn `UserConstructionScript`)