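; Laser-sight pistol weapon that fires hitscan shots and shows a beam stretched to whatever it points at.
; PullTrigger spends ammo via DecrementAmmo, then plays the shot sound, line-traces along FireDirection, spawns sparks and applies point damage.
; Each Tick, on authority only, a second trace from BPLaserSight sets SightScale and rescales the beam's Z axis to reach the hit point.
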(event `self.PullTrigger`
  (params (Instigator :type "Controller Object Reference"))
  (bind _firedirection (`self.FireDirection`))
  (bind _return_value (`self.DecrementAmmo`))
  (if _return_value
    (`GameplayStatics.PlaySoundAtLocation` "/Game/Sounds/lasersightpistol_shot_Cue.lasersightpistol_shot_Cue" (`SceneComponent.K2_GetComponentLocation` (`self.DefaultSceneRoot`)) (struct) 1.0 1.0 0.0 null null null)
    (bind _outhit (`KismetSystemLibrary.LineTraceSingleForObjects` (`SceneComponent.K2_GetComponentLocation` _firedirection) (+ (`SceneComponent.K2_GetComponentLocation` (`self.FireDirection`)) (* (`SceneComponent.GetForwardVector` _firedirection) 2000.0)) (`|MakeArray` "ObjectTypeQuery3" "ObjectTypeQuery2" "ObjectTypeQuery1" :!type "EObjectTypeQuery Enum")))
    (bind (_bblockinghit _binitialoverlap _time _distance _location _impactpoint _normal _impactnormal _physmat _hitactor) (`GameplayStatics.BreakHitResult` _outhit))
    (`GameplayStatics.SpawnEmitterAtLocation` "/Game/StarterContent/Particles/BulletSparks.BulletSparks" _location)
    (`GameplayStatics.ApplyPointDamage` _hitactor 20.0 _location _outhit Instigator)))

(event `self.ReceiveTick`
  (params (DeltaSeconds :type "Float (single-precision)"))
  (`parent.ReceiveTick` DeltaSeconds)
  (`self.LineTraceLaserEndpoint`))

(fn `LineTraceLaserEndpoint`
  (bind _bp_lasersight (`self.BP_LaserSight`))
  (bind _returnvalue (`SceneComponent.K2_GetComponentLocation` _bp_lasersight))
  (`/Engine/EditorBlueprintResources/ActorMacros.Switch Has Authority`
    (:`Authority`
      (bind _outhit (`KismetSystemLibrary.LineTraceSingleForObjects` _returnvalue (+ (* (`SceneComponent.GetUpVector` _bp_lasersight) 10000.0) _returnvalue) (`|MakeArray` "ObjectTypeQuery1" "ObjectTypeQuery3" "ObjectTypeQuery2" :!type "EObjectTypeQuery Enum")))
      (bind (_bblockinghit _binitialoverlap _time _distance _location _impactpoint _normal _impactnormal _physmat _hitactor _hitcomponent _hitbonename _hititem _faceindex _tracestart) (`GameplayStatics.BreakHitResult` _outhit))
      (bind _returnvalue_2 (/ (`KismetMathLibrary.VSize` (- _location _tracestart)) 99.5))
      (set `self.SightScale` _returnvalue_2)
      (`SceneComponent.SetWorldScale3D` (`self.BP_LaserSight`) (`KismetMathLibrary.MakeVector` 0.1 0.1 _returnvalue_2)))))

(fn `UserConstructionScript`
  (`parent.UserConstructionScript`))