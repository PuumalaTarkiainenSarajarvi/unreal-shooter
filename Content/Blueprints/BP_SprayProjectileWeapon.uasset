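; Automatic spray weapon that fires bullet projectiles with a wide random pitch spread.
; Pulling the trigger fires at once and starts a looping timer at the rounds-per-second rate, guarded by a DoOnce that release resets while clearing the timer.
; Each shot spends ammo, spawns a projectile at the spawn point and plays a gunshot, except under the main menu game mode, where it stays silent.
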(event `self.PullTrigger`
  (params (Instigator :type "Controller Object Reference"))
  ;[1 1 1] Trigger pulling & releasing timer logic
  (`/Engine/EditorBlueprintResources/StandardMacros.DoOnce` false :!label _label
    (:`Completed`
      (`self.FireWeapon`)
      (`KismetSystemLibrary.K2_SetTimer` null "FireWeapon" (/ 1.0 (`self.RoundsPerSecond`)) true))))

(event `self.ReleaseTrigger`
  ;[1 1 1] Trigger pulling & releasing timer logic
  (`KismetSystemLibrary.K2_ClearTimer` null "FireWeapon")
  (goto _label :!via `Reset`))

(event `FireWeapon`
  (bind _returnvalue_location (`KismetMathLibrary.BreakTransform` (`self.GetTransform`)))
  (bind _returnvalue (`SceneComponent.K2_GetComponentToWorld` (`self.ProjectileSpawnPoint`)))
  ;[1 1 1] Weapon firing & spawning projectile
  (bind _return_value (`self.DecrementAmmo`))
  (if _return_value
    (`|SpawnActorFromClass` "/Game/Blueprints/BP_BulletProjectile.BP_BulletProjectile_C" (`KismetMathLibrary.MakeTransform` (.location _returnvalue) (`KismetMathLibrary.MakeRotator` (.roll (.rotation _returnvalue)) (+ (.pitch (.rotation _returnvalue)) (`KismetMathLibrary.RandomFloatInRange` -20.0 20.0)) (.yaw (.rotation _returnvalue))) (.scale _returnvalue)) "Undefined" "OverrideRootScale" null null)
    (cast `/Game/Blueprints/BP_MainMenuGamemode` (`GameplayStatics.GetGameMode`)
      (:`CastFailed`
        (`GameplayStatics.PlaySoundAtLocation` "/Game/Sounds/gunshot.gunshot" _returnvalue_location (struct) 1.0 1.0 0.0 null null null)))))

(fn `UserConstructionScript`
  (`parent.UserConstructionScript`)
  (set `self.Ammo` 50))