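; Missile projectile actor that explodes on overlap and deals radial damage.
; On begin play it attaches a spark trail emitter to its mesh.
; Overlapping any actor other than another missile spawns an explosion effect and sound, then destroys the missile.
; Falloff radial damage is applied only when the instigator controller is valid, crediting that controller.
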(event `self.ReceiveBeginPlay`
  (`GameplayStatics.SpawnEmitterAttached` "/Game/StarterContent/Particles/MissileSparks.MissileSparks" (`self.ProjectileMesh`) "None" (0.0 0.0 0.0) (struct) (1.0 1.0 1.0) "SnapToTarget"))

(event `self.ReceiveActorBeginOverlap`
  (params (OtherActor :type "Actor Object Reference"))
  (bind _returnvalue (`self.GetInstigatorController`))
  (bind _returnvalue_location (`KismetMathLibrary.BreakTransform` (`self.GetTransform`)))
  ;[1 1 1] Destroy if hit any actor, deal damage if appropriate
  (cast `/Game/Blueprints/BP_MissileProjectile` OtherActor
    (:`CastFailed`
      (`GameplayStatics.SpawnEmitterAtLocation` "/Game/StarterContent/Particles/P_Explosion.P_Explosion" _returnvalue_location (struct) (4.0 4.0 4.0))
      (`GameplayStatics.PlaySoundAtLocation` "/Game/StarterContent/Audio/Explosion01.Explosion01" _returnvalue_location (struct) 1.0 1.0 0.0 null null null)
      (if (`KismetSystemLibrary.IsValid` _returnvalue)
        (`GameplayStatics.ApplyRadialDamageWithFalloff` :`BaseDamage` 100.0 :`MinimumDamage` 1.0 :`Origin` _returnvalue_location :`DamageInnerRadius` 100.0 :`DamageOuterRadius` 500.0 :`DamageFalloff` 2.0 :`DamageCauser` self :`InstigatedByController` _returnvalue))
      (`self.K2_DestroyActor`))))

(fn `UserConstructionScript`)