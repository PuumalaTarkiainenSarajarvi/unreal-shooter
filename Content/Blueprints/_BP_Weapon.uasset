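; Base-style weapon actor that fires BP_Projectile from a spawn point, automatically while the trigger is held.
; PullTrigger fires once through a DoOnce, then loops a timer at RoundsPerSecond; ReleaseTrigger clears and resets it.
; Each shot plays a laser sound except under the main menu game mode.
; BeginPlay routes laser sight spawning through server and multicast events, but the multicast is empty and the attach logic is disconnected.
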(event `MultiSpawnLaser`)

(event `ServerSpawnLaser`
  (`self.MultiSpawnLaser`))

(event `self.ReceiveBeginPlay`
  (`/Engine/EditorBlueprintResources/ActorMacros.Switch Has Authority`
    (:`Authority`
      (`self.MultiSpawnLaser`))
    (:`Remote`
      (`self.ServerSpawnLaser`))))

(event `self.PullTrigger`
  (params (Instigator :type "Controller Object Reference"))
  ;[1 1 1] Trigger pulling & releasing timer logic
  (`/Engine/EditorBlueprintResources/StandardMacros.DoOnce` false :!label _label
    (:`Completed`
      (`self.FireWeapon`)
      (`KismetSystemLibrary.K2_SetTimer` null "FireWeapon" (/ 1.0 (`self.RoundsPerSecond`)) true))))

(event `ReleaseTrigger`
  ;[1 1 1] Trigger pulling & releasing timer logic
  (`KismetSystemLibrary.K2_ClearTimer` null "FireWeapon")
  (goto _label :!via `Reset`))

(event `FireWeapon`
  (bind _returnvalue_location (`KismetMathLibrary.BreakTransform` (`self.GetTransform`)))
  ;[1 1 1] Weapon firing & spawning projectile
  (`|SpawnActorFromClass` "/Game/Blueprints/BP_Projectile.BP_Projectile_C" (`SceneComponent.K2_GetComponentToWorld` (`self.ProjectileSpawnPoint`)) "Undefined" "OverrideRootScale" null null)
  (cast `/Game/Blueprints/BP_MainMenuGamemode` (`GameplayStatics.GetGameMode`)
    (:`CastFailed`
      (`GameplayStatics.PlaySoundAtLocation` "/Game/Sounds/laser.laser" _returnvalue_location (struct) 1.0 1.0 0.0 null null null))))

(fn `UserConstructionScript`)