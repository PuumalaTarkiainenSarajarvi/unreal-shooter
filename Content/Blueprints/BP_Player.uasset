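; Player Blueprint that rotates SpringArm2's roll to follow the mouse cursor and shows the aim angle in a BP_InfoUI widget.
; Each tick, CalculateDegreeFromCursor derives the angle from screen-space cursor and Cube positions using arctangent with 180-degree quadrant corrections.
; Left click fires a debug line trace from the Arrow and prints the hit actor.
; A Pää hit handler prints test text, and unused experiments and an empty DegreesFromRight remain.
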(event `Key|LeftMouseButton`
  (params (Key :type "Key Structure"))
  (:`Pressed`
    (bind _outhit (`KismetSystemLibrary.LineTraceSingle` :`Start` (`SceneComponent.K2_GetComponentLocation` (`self.Arrow`)) :`End` (+ (`SceneComponent.K2_GetComponentLocation` (`self.Cube`)) (* (`SceneComponent.GetForwardVector` (`self.Arrow`)) 2000.0)) :`TraceChannel` "TraceTypeQuery1" :`DrawDebugType` "ForDuration"))
    (`KismetSystemLibrary.PrintString` (`KismetSystemLibrary.GetDisplayName` (`.HitActor` (`GameplayStatics.BreakHitResult` _outhit))))))

(event `self.ReceiveBeginPlay`
  (bind _returnvalue (`GameplayStatics.GetPlayerController` 0))
  (bind _returnvalue_2 (`|CreateWidget` "/Game/Blueprints/BP_InfoUI.BP_InfoUI_C"))
  (bind _output_get (set `self.InfoUI` _returnvalue_2))
  (`UserWidget.AddToViewport` _output_get 0)
  (`WidgetBlueprintLibrary.SetInputMode_GameAndUIEx` _returnvalue null)
  (set `PlayerController.bShowMouseCursor` true _returnvalue))

(event `self.ReceiveTick`
  (params (DeltaSeconds :type "Float (single-precision)"))
  (bind _returnvalue (`GameplayStatics.GetPlayerController` 0))
  (bind _infoui (`self.InfoUI`))
  ;[1 1 1] Set aside for now
  (bind _angledeg (`self.CalculateDegreeFromCursor` (`PlayerController.ProjectWorldLocationToScreen` _returnvalue (`PlayerController.DeprojectMousePositionToWorld` _returnvalue) true) (`GameplayStatics.ProjectWorldToScreen` _returnvalue (`SceneComponent.K2_GetComponentLocation` (`self.Cube`)))))
  (`SceneComponent.K2_SetWorldRotation` (`self.SpringArm2`) (`KismetMathLibrary.MakeRotator` (* _angledeg -1.0)) false false)
  (cast `/Game/Blueprints/BP_InfoUI` (`self.InfoUI`))
  (`TextBlock.SetText` (`/Game/Blueprints/BP_InfoUI.Rotation` _infoui) "")
  (`TextBlock.SetText` (`/Game/Blueprints/BP_InfoUI.Vector` _infoui) (`KismetTextLibrary.Conv_DoubleToText` _angledeg "HalfToEven")))

(event `self.Pää.OnComponentHit`
  (params (HitComponent :type "PrimitiveComponent Object Reference") (OtherActor :type "Actor Object Reference") (OtherComp :type "PrimitiveComponent Object Reference") (NormalImpulse :type "Vector Structure") (Hit :type "HitResult Structure (by ref)"))
  (`KismetSystemLibrary.PrintString` "Hello"))

(fn `CalculateDegreeFromCursor`
  (params (MouseLocation :type "Vector2D Structure") (ActorLocation :type "Vector2D Structure"))
  (returns (AngleDeg :type "Float (double-precision)"))
  (locals (MouseXCord :type "Float (double-precision)" :default 0.0) (MouseYCord :type "Float (double-precision)" :default 0.0) (ObjectXCord :type "Float (double-precision)" :default 0.0) (ObjectYCord :type "Float (double-precision)" :default 0.0))
  (bind _mousexcord (`local.MouseXCord`))
  (bind _objectxcord (`local.ObjectXCord`))
  (bind _x (.x (`KismetMathLibrary.Conv_Vector2DToVector` MouseLocation)))
  (bind _x_2 (.x (`KismetMathLibrary.Conv_Vector2DToVector` ActorLocation)))
  (bind _returnvalue (/ (* (`KismetMathLibrary.Atan` (/ (- _mousexcord _objectxcord) (- (`local.ObjectYCord`) (`local.MouseYCord`)))) 180.0) (`KismetMathLibrary.GetPI`)))
  (set `local.MouseXCord` _x)
  (set `local.MouseYCord` (.y (`KismetMathLibrary.Conv_Vector2DToVector` MouseLocation)))
  (set `local.ObjectXCord` _x_2)
  (set `local.ObjectYCord` (.y (`KismetMathLibrary.Conv_Vector2DToVector` ActorLocation)))
  (if (< _x _x_2)
    (if (and (> _returnvalue 0.0) (< _mousexcord _objectxcord))
      (return (- _returnvalue 180.0))
      (else
        (return _returnvalue)))
    (elif (and (> _mousexcord _objectxcord) (< _returnvalue 0.0))
      (return (+ _returnvalue 180.0))
      (else
        (return _returnvalue)))))

(fn `DegreesFromRight`
  (params (MouseXcord :type "Float (double-precision)") (MouseYcord :type "Float (double-precision)") (ObjectXcord :type "Float (double-precision)") (ObjectYcord :type "Float (double-precision)"))
  (return))

(fn `UserConstructionScript`)