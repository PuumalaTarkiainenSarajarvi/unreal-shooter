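; BP_DamageTakingObject is an actor with a Health value shown on a TextRender component, set when play begins.
; Its DamageTaken event calls TakeDamage, which subtracts damage from Health and refreshes the displayed text.
; When the result reaches zero or below, Health clamps to zero, IsAlive becomes false and "Dead" is printed.
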(event `self.ReceiveBeginPlay`
  (`TextRenderComponent.K2_SetText` (`self.TextRender`) (`KismetTextLibrary.Conv_DoubleToText` (`self.Health`) "HalfToEven")))

(event `DamageTaken`
  (params (DamageTaken :type "Float (double-precision)"))
  (`self.TakeDamage` DamageTaken))

(fn `TakeDamage`
  (params (DamageTaken :type "Float (double-precision)"))
  (bind _returnvalue (- (`self.Health`) DamageTaken))
  (`/Engine/EditorBlueprintResources/StandardMacros.CompareFloat` _returnvalue
    (:`>`
      (bind _output_get (set `self.Health` _returnvalue)))
    (:`==`
      (set `self.Health` 0.0 :!label _label)
      (set `self.IsAlive` false)
      (`KismetSystemLibrary.PrintString` "Dead"))
    (:`<`
      (goto _label)))
  (`TextRenderComponent.K2_SetText` (`self.TextRender`) (`KismetTextLibrary.Conv_DoubleToText` _output_get "HalfToEven")))

(fn `UserConstructionScript`)