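; BP_LaserSight is a laser sight actor whose length follows the first surface or pawn in its path.
; Every tick it runs an object line trace from the root along its up vector against world static, world dynamic and pawn objects.
; It then rescales the root's Z axis from the trace-start-to-hit distance, keeping a thin fixed X and Y scale.
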(event `self.ReceiveTick`
  (params (DeltaSeconds :type "Float (single-precision)"))
  (`self.LineTraceLaserEndpoint`))

(fn `LineTraceLaserEndpoint`
  (bind _defaultsceneroot (`self.DefaultSceneRoot`))
  (bind _returnvalue (`SceneComponent.K2_GetComponentLocation` _defaultsceneroot))
  (bind _outhit (`KismetSystemLibrary.LineTraceSingleForObjects` _returnvalue (+ (* (`SceneComponent.GetUpVector` _defaultsceneroot) 10000.0) _returnvalue) (`|MakeArray` "ObjectTypeQuery1" "ObjectTypeQuery3" "ObjectTypeQuery2" :!type "EObjectTypeQuery Enum")))
  (bind (_bblockinghit _binitialoverlap _time _distance _location _impactpoint _normal _impactnormal _physmat _hitactor _hitcomponent _hitbonename _hititem _faceindex _tracestart) (`GameplayStatics.BreakHitResult` _outhit))
  (`SceneComponent.SetWorldScale3D` (`self.DefaultSceneRoot`) (`KismetMathLibrary.MakeVector` 0.2 0.2 (/ (`KismetMathLibrary.VSize` (- _location _tracestart)) 99.5))))

(fn `UserConstructionScript`)